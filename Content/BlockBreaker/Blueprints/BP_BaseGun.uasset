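; BP_BaseGun is the base weapon for BlockBreaker, holding a projectile class and a damage value exposed through GetDamage.
; Shoot line-traces on Visibility and spawns a gun-owned projectile, passing the hit point, or trace end on a miss, to MakeSpawnTransform.
; That helper contains ShootSocket look-at math, shown as unused, and Shoot's direct ApplyDamage branch never runs.
; Equipping disables physics simulation on the gun mesh, and unequipping re-enables it.
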(event EventBeginPlay)

(event Collision|EventActorBeginOverlap
  (params (OtherActor :type Actor%20Object%20Reference)))

(event EventTick
  (params (DeltaSeconds :type Float%20%28single-precision%29)))

(fn ConstructionScript)

(fn Shoot
  (params (StartLocation :type Vector) (EndLocation :type Vector))
  (bind _self self)
  (bind _projectile (Variables|Default|GetProjectile))
  (bind (_outhit _returnvalue) (Collision|LineTraceByChannel StartLocation EndLocation "TraceTypeQuery1" false 0 "None"))
  (if _returnvalue
    (Game|SpawnActorfromClass _projectile (Utilities|MakeSpawnTransform (.Location (Collision|BreakHitResult _outhit))) "Undefined" _self 0)
    (else
      (Game|SpawnActorfromClass _projectile (Utilities|MakeSpawnTransform EndLocation) "Undefined" _self 0))))

(fn Equipped
  (Physics|SetSimulatePhysics (Variables|Default|GetGunMesh) false))

(fn Unequipped
  (Physics|SetSimulatePhysics (Variables|Default|GetGunMesh) true))

(fn GetDamage
  (return (Variables|Default|GetDamage)))