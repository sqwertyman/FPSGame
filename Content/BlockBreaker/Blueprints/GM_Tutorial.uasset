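; GM_Tutorial is a BlockBreaker game mode that owns the HUD widgets for aiming and guns.
; On BeginPlay it adds a reticle, an initially hidden pickup prompt and an equipped-gun display to the viewport.
; UpdatePickupUI shows the prompt with the gun's name when given a valid gun and hides it otherwise.
; UpdateGunUI passes the given gun to the equipped-gun widget.
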(event EventBeginPlay
  (bind _returnvalue (UserInterface|CreateWidget "/Game/BlockBreaker/UI/WBP_Reticle.WBP_Reticle_C"))
  (UserInterface|Viewport|AddtoViewport _returnvalue 0)
  (bind _returnvalue_2 (UserInterface|CreateWidget "/Game/BlockBreaker/UI/WBP_Pickup.WBP_Pickup_C"))
  (bind _output_get (Variables|Default|SetPickupGunUI _returnvalue_2))
  (UserInterface|Viewport|AddtoViewport _output_get 0)
  (Widget|SetVisibility _output_get "Hidden")
  (bind _returnvalue_3 (UserInterface|CreateWidget "/Game/BlockBreaker/UI/WBP_EquippedGun.WBP_EquippedGun_C"))
  (bind _output_get_2 (Variables|Default|SetGunUI _returnvalue_3))
  (UserInterface|Viewport|AddtoViewport _output_get_2 0))

(fn ConstructionScript)

(fn UpdatePickupUI
  (params (Gun :type BP%20Base%20Gun%20Object%20Reference))
  (bind _pickupgunui (Variables|Default|GetPickupGunUI))
  (if (Utilities|IsValid Gun)
    (Default|SetGunName _pickupgunui (Variables|/Game/BlockBreaker/Blueprints/Guns/BP_BaseGun.BP_BaseGun_C|GetName Gun))
    (Widget|SetVisibility _pickupgunui "Visible")
    (else
      (Widget|SetVisibility _pickupgunui "Hidden"))))

(fn UpdateGunUI
  (params (gun :type BP%20Base%20Gun%20Object%20Reference))
  (Default|SetGun (Variables|Default|GetGunUI) gun))