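; Base Blueprint for battery-powered guns in BlockBreaker, adding battery and heat limits to its parent gun class.
; Each shot drains battery and adds heat, while Tick cools the gun over time.
; Exceeding max heat clamps it and sets an Overheated lockout that clears only once heat falls to zero.
; CheckCanShoot combines the parent check with remaining battery and the overheat state.
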(event EventBeginPlay
  (|CallParentFunction) ; This node is disabled and will not be called.\nDrag off pins to build functionality.
)

(event Collision|EventActorBeginOverlap
  (params (OtherActor :type Actor%20Object%20Reference))
  (|CallParentFunction OtherActor) ; This node is disabled and will not be called.\nDrag off pins to build functionality.
)

(event EventTick
  (params (DeltaSeconds :type Float%20%28single-precision%29))
  ;[1 1 1] Overheating/cooling
  ;;[1 1 1 1 15] Check for overheat and set if so
  (|CallParentFunction DeltaSeconds)
  (if (> (Variables|Default|GetHeatLevel) (Variables|Default|GetMaxHeat))
    (Variables|Default|SetHeatLevel (Variables|Default|GetMaxHeat))
    (Variables|Default|SetOverheated true)
    (else
      ;;[1 1 1 1 15] Check for cooled down and set if so
      (if (and (Variables|Default|GetOverheated) (<= (Variables|Default|GetHeatLevel) 0.0))
        (Variables|Default|SetOverheated false))))
  (Utilities|DecreaseHeat DeltaSeconds))

(fn ConstructionScript
  (|CallParentFunction))

(fn CheckCanShoot
  (bind _newcanshoot (|CallParentFunction))
  (return (Math|Boolean|ANDBoolean (> (Variables|Default|GetBatteryLevel) 0.0) (not (Variables|Default|GetOverheated)) _newcanshoot)))

(fn HasShot
  (|CallParentFunction)
  (Variables|Default|SetBatteryLevel (- (Variables|Default|GetBatteryLevel) (Variables|Default|GetBatteryUsage)))
  (Variables|Default|SetHeatLevel (+ (Variables|Default|GetHeatLevel) (Variables|Default|GetHeatUsage)))
  (return))